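; Door actor Blueprint that the player opens and closes through an Interact2 event, noted as a press of E.
; Interact2 toggles DoorOpen and plays or reverses a timeline whose DoorAngle track drives the Door's relative yaw.
; A P_Interact prompt widget, created on BeginPlay, is shown while the player character overlaps InteractionBox and removed when they leave.
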(event `/Game/BPs/BPI_Interact.Interact2`
  ; Door event to close and open on press E
  (if (not (`self.DoorOpen?`))
    (set `self.DoorOpen?` true)
    (bind (_direction _doorangle) (`Timeline|OpenCloseTimeline` :!label _label)
      (:`Update`
        (`SceneComponent.K2_SetRelativeRotation` (`self.Door`) (`KismetMathLibrary.MakeRotator` 0.0 0.0 _doorangle) false false)))
    (else
      (set `self.DoorOpen?` false)
      (goto _label :!via `Reverse`))))

(event `self.InteractionBox.OnComponentBeginOverlap`
  (params (OverlappedComponent :type "PrimitiveComponent Object Reference") (OtherActor :type "Actor Object Reference") (OtherComp :type "PrimitiveComponent Object Reference") (OtherBodyIndex :type Integer) (bFromSweep :type Boolean) (SweepResult :type "HitResult Structure (by ref)"))
  ; Interact text pop
  (if (== OtherActor (`GameplayStatics.GetPlayerCharacter` 0))
    ;; sub setup calling the prompt
    (`UserWidget.AddToViewport` (`self.Interact Prompt`) 0)))

(event `self.ReceiveBeginPlay`
  ; Interact text pop
  (bind _returnvalue (`|CreateWidget` "/Game/BPs/P_Interact.P_Interact_C"))
  (set `self.Interact Prompt` _returnvalue))

(event `self.InteractionBox.OnComponentEndOverlap`
  (params (OverlappedComponent :type "PrimitiveComponent Object Reference") (OtherActor :type "Actor Object Reference") (OtherComp :type "PrimitiveComponent Object Reference") (OtherBodyIndex :type Integer))
  ; Interact text pop
  (if (== (`GameplayStatics.GetPlayerCharacter` 0) OtherActor)
    ;; sub setup calling the prompt
    (`Widget.RemoveFromParent` (`self.Interact Prompt`))))

(fn `UserConstructionScript`
  (`parent.UserConstructionScript`))